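; Game mode for a rocket jump game that sets up the extraction point and runs the match countdown.
; BeginPlay spawns an ExtractionPoint at a hard-coded location, disables its collision, hides its sphere, and switches the player to game-only input without a cursor.
; Tick uses a one-second Delay as a timer to decrement Seconds and Minutes, pausing the game when time runs out.
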(event EventTick
  (params (DeltaSeconds :type Float%20%28single-precision%29))
  (Utilities|FlowControl|Delay 1.0)
  (Variables|Default|SetSeconds (- (Variables|Default|GetSeconds) 1))
  (if (< (Variables|Default|GetSeconds) 0)
    (Variables|Default|SetSeconds 59)
    (Variables|Default|SetMinutes (- (Variables|Default|GetMinutes) 1))
    (if (< (Variables|Default|GetMinutes) 0)
      (Game|SetGamePaused true))))

(event EventBeginPlay
  (bind _returnvalue (Game|GetPlayerController 0))
  (bind _returnvalue_2 (Game|SpawnActorfromClass "/Game/Arbetsprov/Blueprints/ExtractionPoint.ExtractionPoint_C" (Math|Transform|MakeTransform "8500.000000,500.000000,1510.000000" "0,180.000000, 0" "1,1,1") "Undefined" 0 0))
  (bind _output_get (Variables|Default|SetExtractionPointRef _returnvalue_2))
  (Collision|SetActorEnableCollision _output_get false)
  (Rendering|SetVisibility (Variables|/Game/Arbetsprov/Blueprints/ExtractionPoint.ExtractionPoint_C|GetSphere _output_get) false false)
  (Variables|/Script/Engine.PlayerController|SetbShowMouseCursor _returnvalue false)
  (Input|SetInputModeGameOnly _returnvalue))

(fn ConstructionScript)