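; Rocket launcher projectile that explodes when it begins overlapping another actor.
; Overlaps with RocketExplosion actors and ArbetsprovCharacter are filtered out by casting and comparing the result to the other actor.
; Any other overlap plays an explosion particle and sound, then passes a DoOnce to spawn a RocketExplosion at its transform and destroy itself.
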(event EventBeginPlay)

(event Collision|EventActorBeginOverlap
  (params (OtherActor :type Actor%20Object%20Reference))
  (bind _asrocket_explosion (Utilities|Casting|CastToRocketExplosion OtherActor)
    (:then
      _)
    (:CastFailed
      _))
  (if (not (== OtherActor _asrocket_explosion))
    (bind _asarbetsprov_character (Utilities|Casting|CastToArbetsprovCharacter OtherActor)
      (:then
        _)
      (:CastFailed
        _))
    (if (not (== OtherActor _asarbetsprov_character))
      (Effects|SpawnEmitteratLocation "/Game/SciFiWeapLight/FX/Particles/P_RocketLauncher_Explosion_Light.P_RocketLauncher_Explosion_Light" (Transformation|GetActorLocation))
      (Audio|SpawnSoundatLocation "/Game/SciFiWeapLight/Sound/RocketLauncher/Wavs/RL_Explosion01.RL_Explosion01" (Transformation|GetActorLocation) "0, 0, 0" 0.3 1.0 0.0 0 0)
      (Utilities|FlowControl|DoOnce false
        (:Completed
          (Game|SpawnActorfromClass "/Game/Arbetsprov/Blueprints/WeaponsAndEH/RocketExplosion.RocketExplosion_C" (Transformation|GetActorTransform) "Undefined" 0 0)
          (Actor|DestroyActor))))))

(event EventTick
  (params (DeltaSeconds :type Float%20%28single-precision%29)))

(fn ConstructionScript)