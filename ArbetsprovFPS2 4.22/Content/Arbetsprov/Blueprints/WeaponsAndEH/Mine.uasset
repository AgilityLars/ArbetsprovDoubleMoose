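; Proximity mine that detonates when the player character or a SimpleAI actor enters its trigger sphere (Sphere1).
; The overlap event casts to ArbetsprovCharacter first, then falls back to SimpleAI, ignoring other actors.
; Detonation spawns a MineExplosion actor at the victim's mesh transform, plays a grenade explosion particle at the mine's Sphere location, then destroys the mine.
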(event OnComponentBeginOverlap(Sphere1)
  (params (OverlappedComponent :type Primitive%20Component%20Object%20Reference) (OtherActor :type Actor%20Object%20Reference) (OtherComp :type Primitive%20Component%20Object%20Reference) (OtherBodyIndex :type Integer) (bFromSweep :type Boolean) (SweepResult :type Hit%20Result%20Structure%20%28by%20ref%29))
  (bind _sphere (Variables|Default|GetSphere))
  (bind _returnvalue (Transformation|GetWorldLocation _sphere))
  (bind _asarbetsprov_character (Utilities|Casting|CastToArbetsprovCharacter OtherActor)
    (:then
      (Game|SpawnActorfromClass "/Game/Arbetsprov/Blueprints/WeaponsAndEH/MineExplosion.MineExplosion_C" (Transformation|GetWorldTransform (Variables|/Script/Engine.Character|GetMesh _asarbetsprov_character)) "Undefined" 0 0)
      (Effects|SpawnEmitteratLocation "/Game/SciFiWeapLight/FX/Particles/P_Grenade_Explosion_Dark.P_Grenade_Explosion_Dark" _returnvalue)
      (Actor|DestroyActor))
    (:CastFailed
      (bind _assimple_ai (Utilities|Casting|CastToSimpleAI OtherActor))
      (Game|SpawnActorfromClass "/Game/Arbetsprov/Blueprints/WeaponsAndEH/MineExplosion.MineExplosion_C" (Transformation|GetWorldTransform (Variables|/Script/Engine.Character|GetMesh _assimple_ai)) "Undefined" 0 0)
      (Effects|SpawnEmitteratLocation "/Game/SciFiWeapLight/FX/Particles/P_Grenade_Explosion_Dark.P_Grenade_Explosion_Dark" _returnvalue)
      (Actor|DestroyActor))))

(event EventBeginPlay)

(event Collision|EventActorBeginOverlap
  (params (OtherActor :type Actor%20Object%20Reference)))

(event EventTick
  (params (DeltaSeconds :type Float%20%28single-precision%29)))

(fn ConstructionScript)