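; SimpleAI is a zombie enemy that wanders randomly, chases the player via pawn sensing and deals melee damage through sphere overlap during timed attack windows.
; Projectile, rocket and mine overlaps reduce health, with bullet and rocket hits drawing it toward the player.
; Rocket and mine deaths ragdoll it, request replacements and advance the kill objective toward extraction; projectile deaths only trigger feedback.
; Under StartMenuGameMode, mine hits instead spawn random replacement zombies or mines.
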(event OnSeePawn(PawnSensing)
  (params (Pawn :type Pawn%20Object%20Reference))
  (bind _asarbetsprov_character (Utilities|Casting|CastToArbetsprovCharacter Pawn))
  (Variables|Default|SetCanSeePlayer true)
  (Variables|/Script/Engine.CharacterMovementComponent|SetMaxWalkSpeed (Variables|Character|GetCharacterMovement) 4e+02)
  (AI|AIMoveTo self "0, 0, 0" _asarbetsprov_character 5.0 false :!label _label
    (:OnSuccess
      (if (not (Variables|Default|GetAttacking))
        (Variables|Default|SetAttacking true)
        (Utilities|FlowControl|Delay 2.3)
        (Variables|Default|SetAttacking false)
        (Variables|Default|SetAlreadyHit false)
        (goto _label)))))

(event OnComponentBeginOverlap(Sphere)
  (params (OverlappedComponent :type Primitive%20Component%20Object%20Reference) (OtherActor :type Actor%20Object%20Reference) (OtherComp :type Primitive%20Component%20Object%20Reference) (OtherBodyIndex :type Integer) (bFromSweep :type Boolean) (SweepResult :type Hit%20Result%20Structure%20%28by%20ref%29))
  (bind _asarbetsprov_character (Utilities|Casting|CastToArbetsprovCharacter OtherActor))
  (if (Variables|Default|GetAttacking)
    (if (not (Variables|Default|GetAlreadyHit))
      (if (not (Variables|Default|GetIsDead))
        (Default|TakeDamageFunction _asarbetsprov_character 0.2)
        (Variables|Default|SetAlreadyHit true)))))

(event Custom|SpawnedZombie
  (AI|AIMoveTo self (.RandomLocation (AI|Navigation|GetRandomReachablePointinRadius (Transformation|GetActorLocation) 1e+04 0 0)) 0 5.0 false :!label _label
    (:OnSuccess
      _)
    (:OnFail
      _))
  (if (not (Variables|Default|GetCanSeePlayer))
    (goto _label)))

(event EventBeginPlay
  (AI|AIMoveTo self (.RandomLocation (AI|Navigation|GetRandomReachablePointinRadius (Transformation|GetActorLocation) 1e+04 0 0)) 0 5.0 false
    (:then
      (Utilities|FlowControl|Delay 2.0)
      (Variables|Default|SetJustSpawned false)
      (AI|AIMoveTo self (.RandomLocation (AI|Navigation|GetRandomReachablePointinRadius (Transformation|GetActorLocation) 1e+04 0 0)) 0 5.0 false :!label _label
        (:OnSuccess
          _)
        (:OnFail
          _))
      (if (not (Variables|Default|GetCanSeePlayer))
        (goto _label)))))

(event Collision|EventActorBeginOverlap
  (params (OtherActor :type Actor%20Object%20Reference))
  (bind _returnvalue (Game|GetGameMode))
  (bind _mesh (Variables|Character|GetMesh))
  (bind _capsulecomponent (Variables|Collision|GetCapsuleComponent))
  (bind _mesh_2 (Variables|Character|GetMesh))
  (bind _capsulecomponent_2 (Variables|Collision|GetCapsuleComponent))
  (bind _mesh_3 (Variables|Character|GetMesh))
  (bind _capsulecomponent_3 (Variables|Collision|GetCapsuleComponent))
  (if (and (Math|Boolean|Equal(Boolean) (Variables|Default|GetIsDead) false) (Math|Boolean|Equal(Boolean) (Variables|Default|GetJustSpawned) false))
    (bind _asprojectile_base (Utilities|Casting|CastToProjectileBase OtherActor)
      (:then
        (Variables|Default|SetHealth (- (Variables|Default|GetHealth) 1e+01))
        (bind _returnvalue_2 (UserInterface|CreateWidget "/Game/Arbetsprov/Blueprints/MenusAndUI/Hitmarker.Hitmarker_C"))
        (UserInterface|Viewport|AddtoViewport _returnvalue_2 0)
        (bind _asarbetsprov_character (Utilities|Casting|CastToArbetsprovCharacter (Game|GetPlayerCharacter 0)))
        (Audio|SpawnSoundatLocation "/Engine/VREditor/Sounds/UI/Object_Snaps_To_Grid.Object_Snaps_To_Grid" (Transformation|GetActorLocation _asarbetsprov_character) "0, 0, 0" 1.0 1.0 0.0 0 0)
        (if (<= (Variables|Default|GetHealth) 0.0)
          (Effects|SpawnEmitteratLocation "/Game/InfinityBladeEffects/Effects/FX_Monsters/FX_Monster_Gruntling/Notifies/P_Death_PickImpact.P_Death_PickImpact" (Transformation|GetActorLocation))
          (Audio|SpawnSoundatLocation "/Engine/EditorSounds/GamePreview/PossessPlayer.PossessPlayer" (Transformation|GetActorLocation) "0, 0, 0" 1.0 1.0 0.0 0 0)
          (bind _returnvalue_3 (UserInterface|CreateWidget "/Game/Arbetsprov/Blueprints/MenusAndUI/KillFeedPopup.KillFeedPopup_C"))
          (UserInterface|Viewport|AddtoViewport _returnvalue_3 0)
          (else
            (Effects|SpawnEmitteratLocation "/Game/InfinityBladeEffects/Effects/FX_Mobile/Impacts/P_Impact_Shield_Fire.P_Impact_Shield_Fire" (Transformation|GetActorLocation _asprojectile_base))
            (bind _asarbetsprov_character_2 (Utilities|Casting|CastToArbetsprovCharacter (Game|GetPlayerCharacter 0)))
            (AI|AIMoveTo self "0, 0, 0" _asarbetsprov_character_2 5.0 false))))
      (:CastFailed
        (bind _asrocket_explosion (Utilities|Casting|CastToRocketExplosion OtherActor)
          (:then
            (Variables|Default|SetHealth (- (Variables|Default|GetHealth) 5e+01))
            (if (<= (Variables|Default|GetHealth) 0.0)
              (Effects|SpawnEmitteratLocation "/Game/InfinityBladeEffects/Effects/FX_Monsters/FX_Monster_Gruntling/Notifies/P_Death_PickImpact.P_Death_PickImpact" (Transformation|GetActorLocation))
              (Audio|SpawnSoundatLocation "/Engine/EditorSounds/GamePreview/PossessPlayer.PossessPlayer" (Transformation|GetActorLocation) "0, 0, 0" 1.0 1.0 0.0 0 0)
              (bind _returnvalue_4 (UserInterface|CreateWidget "/Game/Arbetsprov/Blueprints/MenusAndUI/KillFeedPopup.KillFeedPopup_C"))
              (UserInterface|Viewport|AddtoViewport _returnvalue_4 0)
              (bind _asarbetsprov_game_mode (Utilities|Casting|CastToArbetsprovGameMode (Game|GetGameMode)))
              (Default|SpawnZombie (Variables|/Game/Arbetsprov/Blueprints/ArbetsprovGameMode.ArbetsprovGameMode_C|GetSpawner1Ref _asarbetsprov_game_mode))
              (Physics|SetSimulatePhysics _mesh_2 true)
              (Variables|/Script/Engine.PrimitiveComponent|SetbGenerateOverlapEvents _mesh_2 false)
              (Collision|SetCollisionEnabled _capsulecomponent_2 "NoCollision")
              (Collision|SetCollisionResponsetoAllChannels _capsulecomponent_2 "ECR_Ignore")
              (Variables|Default|SetIsDead true)
              (bind _asarbetsprov_character_3 (Utilities|Casting|CastToArbetsprovCharacter (Game|GetPlayerCharacter 0)))
              (if (Utilities|Enum|Equal(Enum) (Variables|/Game/Arbetsprov/Blueprints/ArbetsprovCharacter.ArbetsprovCharacter_C|GetObjectiveEnum _asarbetsprov_character_3) "NewEnumerator0")
                (Variables|/Game/Arbetsprov/Blueprints/ArbetsprovCharacter.ArbetsprovCharacter_C|SetObjectiveKillsNeeded _asarbetsprov_character_3 (- (Variables|/Game/Arbetsprov/Blueprints/ArbetsprovCharacter.ArbetsprovCharacter_C|GetObjectiveKillsNeeded _asarbetsprov_character_3) 1))
                (if (<= (Variables|/Game/Arbetsprov/Blueprints/ArbetsprovCharacter.ArbetsprovCharacter_C|GetObjectiveKillsNeeded _asarbetsprov_character_3) 0)
                  (Variables|/Game/Arbetsprov/Blueprints/ArbetsprovCharacter.ArbetsprovCharacter_C|SetObjectiveEnum _asarbetsprov_character_3 "NewEnumerator1")
                  (bind _asarbetsprov_game_mode_2 (Utilities|Casting|CastToArbetsprovGameMode (Game|GetGameMode)))
                  (Collision|SetActorEnableCollision (Variables|/Game/Arbetsprov/Blueprints/ArbetsprovGameMode.ArbetsprovGameMode_C|GetExtractionPointRef _asarbetsprov_game_mode_2) true)
                  (Rendering|SetVisibility (Variables|/Game/Arbetsprov/Blueprints/ExtractionPoint.ExtractionPoint_C|GetSphere (Variables|/Game/Arbetsprov/Blueprints/ArbetsprovGameMode.ArbetsprovGameMode_C|GetExtractionPointRef _asarbetsprov_game_mode_2)) true false)))
              (else
                (Effects|SpawnEmitteratLocation "/Game/InfinityBladeEffects/Effects/FX_Mobile/Impacts/P_Impact_Shield_Fire.P_Impact_Shield_Fire" (Transformation|GetActorLocation _asrocket_explosion))
                (bind _asarbetsprov_character_4 (Utilities|Casting|CastToArbetsprovCharacter (Game|GetPlayerCharacter 0)))
                (AI|AIMoveTo self "0, 0, 0" _asarbetsprov_character_4 5.0 false))))
          (:CastFailed
            (bind _asmine_explosion (Utilities|Casting|CastToMineExplosion OtherActor))
            (Variables|Default|SetHealth (- (Variables|Default|GetHealth) 5e+01))
            (Utilities|Casting|CastToArbetsprovGameMode _returnvalue
              (:then
                (if (<= (Variables|Default|GetHealth) 0.0)
                  (Effects|SpawnEmitteratLocation "/Game/InfinityBladeEffects/Effects/FX_Monsters/FX_Monster_Gruntling/Notifies/P_Death_PickImpact.P_Death_PickImpact" (Transformation|GetActorLocation))
                  (bind _returnvalue_5 (UserInterface|CreateWidget "/Game/Arbetsprov/Blueprints/MenusAndUI/KillFeedPopup.KillFeedPopup_C"))
                  (UserInterface|Viewport|AddtoViewport _returnvalue_5 0)
                  (bind _asarbetsprov_game_mode_3 (Utilities|Casting|CastToArbetsprovGameMode (Game|GetGameMode))
                    (:then
                      (Default|SpawnZombie (Variables|/Game/Arbetsprov/Blueprints/ArbetsprovGameMode.ArbetsprovGameMode_C|GetSpawner1Ref _asarbetsprov_game_mode_3)))
                    (:CastFailed
                      _))
                  (Physics|SetSimulatePhysics _mesh_3 true)
                  (Variables|/Script/Engine.PrimitiveComponent|SetbGenerateOverlapEvents _mesh_3 false)
                  (Collision|SetCollisionEnabled _capsulecomponent_3 "NoCollision")
                  (Collision|SetCollisionResponsetoAllChannels _capsulecomponent_3 "ECR_Ignore")
                  (Variables|Default|SetIsDead true)
                  (bind _asarbetsprov_character_5 (Utilities|Casting|CastToArbetsprovCharacter (Game|GetPlayerCharacter 0)))
                  (if (Utilities|Enum|Equal(Enum) (Variables|/Game/Arbetsprov/Blueprints/ArbetsprovCharacter.ArbetsprovCharacter_C|GetObjectiveEnum _asarbetsprov_character_5) "NewEnumerator0")
                    (Variables|/Game/Arbetsprov/Blueprints/ArbetsprovCharacter.ArbetsprovCharacter_C|SetObjectiveKillsNeeded _asarbetsprov_character_5 (- (Variables|/Game/Arbetsprov/Blueprints/ArbetsprovCharacter.ArbetsprovCharacter_C|GetObjectiveKillsNeeded _asarbetsprov_character_5) 1))
                    (if (<= (Variables|/Game/Arbetsprov/Blueprints/ArbetsprovCharacter.ArbetsprovCharacter_C|GetObjectiveKillsNeeded _asarbetsprov_character_5) 0)
                      (Variables|/Game/Arbetsprov/Blueprints/ArbetsprovCharacter.ArbetsprovCharacter_C|SetObjectiveEnum _asarbetsprov_character_5 "NewEnumerator1")
                      (bind _asarbetsprov_game_mode_4 (Utilities|Casting|CastToArbetsprovGameMode (Game|GetGameMode)))
                      (Collision|SetActorEnableCollision (Variables|/Game/Arbetsprov/Blueprints/ArbetsprovGameMode.ArbetsprovGameMode_C|GetExtractionPointRef _asarbetsprov_game_mode_4) true)
                      (Rendering|SetVisibility (Variables|/Game/Arbetsprov/Blueprints/ExtractionPoint.ExtractionPoint_C|GetSphere (Variables|/Game/Arbetsprov/Blueprints/ArbetsprovGameMode.ArbetsprovGameMode_C|GetExtractionPointRef _asarbetsprov_game_mode_4)) true false)))
                  (else
                    (Effects|SpawnEmitteratLocation "/Game/InfinityBladeEffects/Effects/FX_Mobile/Impacts/P_Impact_Shield_Fire.P_Impact_Shield_Fire" (Transformation|GetActorLocation _asmine_explosion)))))
              (:CastFailed
                (Utilities|Casting|CastToStartMenuGameMode _returnvalue)
                (if (<= (Variables|Default|GetHealth) 0.0)
                  (Effects|SpawnEmitteratLocation "/Game/InfinityBladeEffects/Effects/FX_Monsters/FX_Monster_Gruntling/Notifies/P_Death_PickImpact.P_Death_PickImpact" (Transformation|GetActorLocation))
                  (Physics|SetSimulatePhysics _mesh true)
                  (Variables|/Script/Engine.PrimitiveComponent|SetbGenerateOverlapEvents _mesh false)
                  (Collision|SetCollisionEnabled _capsulecomponent "NoCollision")
                  (Collision|SetCollisionResponsetoAllChannels _capsulecomponent "ECR_Ignore")
                  (Variables|Default|SetIsDead true)
                  (Game|SpawnActorfromClass "SimpleAI_C" (Math|Transform|MakeTransform (Math|Vector|MakeVector (Math|Random|RandomFloatinRange -1.8e+03 1e+03) (Math|Random|RandomFloatinRange -1.4e+03 1.4e+03) 4e+02)) "Undefined" 0 0)
                  (else
                    (Effects|SpawnEmitteratLocation "/Game/InfinityBladeEffects/Effects/FX_Mobile/Impacts/P_Impact_Shield_Fire.P_Impact_Shield_Fire" (Transformation|GetActorLocation))
                    (Game|SpawnActorfromClass "/Game/Arbetsprov/Blueprints/WeaponsAndEH/Mine.Mine_C" (Math|Transform|MakeTransform (Math|Vector|MakeVector (Math|Random|RandomFloatinRange -1.8e+03 1e+03) (Math|Random|RandomFloatinRange -1.4e+03 1.4e+03) 4e+02)) "Undefined" 0 0)))))))))))

(fn ConstructionScript)