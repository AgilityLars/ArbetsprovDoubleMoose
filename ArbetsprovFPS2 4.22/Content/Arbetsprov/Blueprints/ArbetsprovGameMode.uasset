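; Game mode that sets up the zombie and extraction level and runs the match countdown.
; BeginPlay spawns a zombie spawner and triggers it, spawns an extraction point with collision off and its sphere hidden, and sets game-only input.
; Tick uses a one-second Delay as a timer to decrement seconds and minutes, pausing the game when time runs out.
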(event EventTick
  (params (DeltaSeconds :type Float%20%28single-precision%29))
  (Utilities|FlowControl|Delay 1.0)
  (Variables|Default|SetSeconds (- (Variables|Default|GetSeconds) 1))
  (if (< (Variables|Default|GetSeconds) 0)
    (Variables|Default|SetSeconds 59)
    (Variables|Default|SetMinutes (- (Variables|Default|GetMinutes) 1))
    (if (< (Variables|Default|GetMinutes) 0)
      (Game|SetGamePaused true))))

(event EventBeginPlay
  (bind _returnvalue (Game|GetPlayerController 0))
  (bind _returnvalue_2 (Game|SpawnActorfromClass "/Game/Arbetsprov/Blueprints/ZombieSpawner.ZombieSpawner_C" (Math|Transform|MakeTransform "865.000000,1275.000000,131.000000" "0,180.000000, 0" "1,1,1") "Undefined" 0 0))
  (bind _output_get (Variables|Default|SetSpawner1Ref _returnvalue_2))
  (Default|SpawnZombie _output_get)
  (bind _returnvalue_3 (Game|SpawnActorfromClass "/Game/Arbetsprov/Blueprints/ExtractionPoint.ExtractionPoint_C" (Math|Transform|MakeTransform "41.000000,-1295.000000,512.000000" "0,180.000000, 0" "1,1,1") "Undefined" 0 0))
  (bind _output_get_2 (Variables|Default|SetExtractionPointRef _returnvalue_3))
  (Collision|SetActorEnableCollision _output_get_2 false)
  (Rendering|SetVisibility (Variables|/Game/Arbetsprov/Blueprints/ExtractionPoint.ExtractionPoint_C|GetSphere _output_get_2) false false)
  (Variables|/Script/Engine.PlayerController|SetbShowMouseCursor _returnvalue false)
  (Input|SetInputModeGameOnly _returnvalue))

(fn ConstructionScript)