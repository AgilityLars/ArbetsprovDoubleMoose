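; M4A1 weapon pickup that grants the rifle to the player character on overlap.
; Overlap with an ArbetsprovCharacter sets its HasM4A1 flag, plays a loot particle and pickup sound, destroys the actor and shows a PickupWidget message.
; Tick spins the weapon component by adding a fixed yaw step to its world transform after a short Delay, so the rotation rate is not scaled by delta time.
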(event EventBeginPlay)

(event Collision|EventActorBeginOverlap
  (params (OtherActor :type Actor%20Object%20Reference))
  (bind _asarbetsprov_character (Utilities|Casting|CastToArbetsprovCharacter OtherActor))
  (Variables|/Game/Arbetsprov/Blueprints/ArbetsprovCharacter.ArbetsprovCharacter_C|SetHasM4A1 _asarbetsprov_character true)
  (Effects|SpawnEmitteratLocation "/Game/InfinityBladeEffects/Effects/FX_Treasure/Loot/P_Loot_Pickup.P_Loot_Pickup" (Transformation|GetActorLocation))
  (Audio|SpawnSoundatLocation "/Engine/VREditor/Sounds/UI/Object_PickUp.Object_PickUp" (Transformation|GetActorLocation) "0, 0, 0" 1.5 1.0 0.0 0 0)
  (Actor|DestroyActor)
  (bind _returnvalue (UserInterface|CreateWidget "/Game/Arbetsprov/Blueprints/Pickups/PickupWidget.PickupWidget_C"))
  (UserInterface|Viewport|AddtoViewport _returnvalue 0)
  (Variables|/Game/Arbetsprov/Blueprints/Pickups/PickupWidget.PickupWidget_C|SetText _returnvalue "Picked up a M4A1"))

(event EventTick
  (params (DeltaSeconds :type Float%20%28single-precision%29))
  (bind _m4a1_weapon002 (Variables|Default|GetM4A1_weapon002))
  (bind _returnvalue (Transformation|GetWorldTransform _m4a1_weapon002))
  (Utilities|FlowControl|Delay 0.02)
  (Transformation|SetWorldTransform _m4a1_weapon002 (Math|Transform|MakeTransform (Math|Vector|MakeVector (.x (.location _returnvalue)) (.y (.location _returnvalue)) (.z (.location _returnvalue))) (Math|Rotator|MakeRotator (.roll (.rotation _returnvalue)) (.pitch (.rotation _returnvalue)) (+ (.yaw (.rotation _returnvalue)) 1.0)) (.scale _returnvalue)) false false))

(fn ConstructionScript)