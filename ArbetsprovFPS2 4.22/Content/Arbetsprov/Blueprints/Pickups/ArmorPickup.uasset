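; Armor pickup that raises the overlapping ArbetsprovCharacter's armor by a fixed step, or sets it to the cap when near or at max.
; Either way it destroys itself, plays a particle and sound, and shows a PickupWidget message, reporting max armor in the capped case.
; Tick, throttled by a short Delay, spins and bobs the mesh between height limits the construction script derives from its placed position.
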(event Collision|EventActorBeginOverlap
  (params (OtherActor :type Actor%20Object%20Reference))
  (Utilities|FlowControl|Delay 0.1)
  (bind _asarbetsprov_character (Utilities|Casting|CastToArbetsprovCharacter OtherActor))
  (if (< (Variables|/Game/Arbetsprov/Blueprints/ArbetsprovCharacter.ArbetsprovCharacter_C|GetArmor _asarbetsprov_character) 1.5)
    (Variables|/Game/Arbetsprov/Blueprints/ArbetsprovCharacter.ArbetsprovCharacter_C|SetArmor _asarbetsprov_character (+ (Variables|/Game/Arbetsprov/Blueprints/ArbetsprovCharacter.ArbetsprovCharacter_C|GetArmor _asarbetsprov_character) 0.5))
    (Actor|DestroyActor)
    (Effects|SpawnEmitteratLocation "/Game/InfinityBladeEffects/Effects/FX_Treasure/Loot/P_Loot_Pickup.P_Loot_Pickup" (Transformation|GetActorLocation))
    (Audio|SpawnSoundatLocation "/Engine/VREditor/Sounds/UI/Object_PickUp.Object_PickUp" (Transformation|GetActorLocation) "0, 0, 0" 1.5 1.0 0.0 0 0)
    (bind _returnvalue (UserInterface|CreateWidget "/Game/Arbetsprov/Blueprints/Pickups/PickupWidget.PickupWidget_C"))
    (UserInterface|Viewport|AddtoViewport _returnvalue 0)
    (Variables|/Game/Arbetsprov/Blueprints/Pickups/PickupWidget.PickupWidget_C|SetText _returnvalue "Picked up an armor pack")
    (else
      (Variables|/Game/Arbetsprov/Blueprints/ArbetsprovCharacter.ArbetsprovCharacter_C|SetArmor _asarbetsprov_character 2.0)
      (Actor|DestroyActor)
      (Effects|SpawnEmitteratLocation "/Game/InfinityBladeEffects/Effects/FX_Treasure/Loot/P_Loot_Pickup.P_Loot_Pickup" (Transformation|GetActorLocation))
      (Audio|SpawnSoundatLocation "/Engine/VREditor/Sounds/UI/Object_PickUp.Object_PickUp" (Transformation|GetActorLocation) "0, 0, 0" 1.5 1.0 0.0 0 0)
      (bind _returnvalue_2 (UserInterface|CreateWidget "/Game/Arbetsprov/Blueprints/Pickups/PickupWidget.PickupWidget_C"))
      (UserInterface|Viewport|AddtoViewport _returnvalue_2 0)
      (Variables|/Game/Arbetsprov/Blueprints/Pickups/PickupWidget.PickupWidget_C|SetText _returnvalue_2 "Your armor is already at max"))))

(event EventTick
  (params (DeltaSeconds :type Float%20%28single-precision%29))
  (bind _staticmesh (Variables|Default|GetStaticMesh))
  (bind _staticmesh_2 (Variables|Default|GetStaticMesh))
  (bind _returnvalue (Transformation|GetWorldTransform _staticmesh))
  (bind _returnvalue_2 (Transformation|GetWorldTransform _staticmesh_2))
  (Utilities|FlowControl|Delay 0.02)
  (if (Variables|Default|GetUp)
    (Transformation|SetWorldTransform _staticmesh_2 (Math|Transform|MakeTransform (Math|Vector|MakeVector (.x (.location _returnvalue_2)) (.y (.location _returnvalue_2)) (+ (.z (.location _returnvalue_2)) 0.5)) (Math|Rotator|MakeRotator (.roll (.rotation _returnvalue_2)) (.pitch (.rotation _returnvalue_2)) (+ (.yaw (.rotation _returnvalue_2)) 1.0)) (.scale _returnvalue_2)) false false)
    (Variables|Default|SetCurrentHeight (.z (.location (Transformation|GetWorldTransform (Variables|Default|GetStaticMesh)))))
    (if (> (Variables|Default|GetCurrentHeight) (Variables|Default|GetMaxHeight))
      (Variables|Default|SetUp false))
    (else
      (Transformation|SetWorldTransform _staticmesh (Math|Transform|MakeTransform (Math|Vector|MakeVector (.x (.location _returnvalue)) (.y (.location _returnvalue)) (- (.z (.location _returnvalue)) 0.5)) (Math|Rotator|MakeRotator (.roll (.rotation _returnvalue)) (.pitch (.rotation _returnvalue)) (+ (.yaw (.rotation _returnvalue)) 1.0)) (.scale _returnvalue)) false false)
      (Variables|Default|SetCurrentHeight (.z (.location (Transformation|GetWorldTransform (Variables|Default|GetStaticMesh)))))
      (if (< (Variables|Default|GetCurrentHeight) (Variables|Default|GetMinHeight))
        (Variables|Default|SetUp true)))))

(fn ConstructionScript
  (bind _staticmesh (Variables|Default|GetStaticMesh))
  (bind _returnvalue (Transformation|GetWorldTransform _staticmesh))
  (Variables|Default|SetCurrentHeight (.z (.location _returnvalue)))
  (Variables|Default|SetMaxHeight (+ (.z (.location _returnvalue)) 2e+01))
  (Variables|Default|SetMinHeight (- (.z (.location _returnvalue)) 2e+01)))