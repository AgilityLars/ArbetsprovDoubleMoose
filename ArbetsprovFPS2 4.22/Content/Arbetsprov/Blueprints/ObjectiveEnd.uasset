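; ObjectiveEnd is an objective pickup that, when the player character overlaps it, advances that character's objective enum and destroys itself.
; It then unlocks extraction by enabling collision and showing the sphere on the game mode's extraction point reference.
; It supports both RocketJumpGameMode and ArbetsprovGameMode through a fallback cast.
; A Delay-gated Tick continually increments the cube's roll to spin it.
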(event EventBeginPlay)

(event Collision|EventActorBeginOverlap
  (params (OtherActor :type Actor%20Object%20Reference))
  (bind _returnvalue (Game|GetGameMode))
  (bind _asarbetsprov_character (Utilities|Casting|CastToArbetsprovCharacter OtherActor))
  (Variables|/Game/Arbetsprov/Blueprints/ArbetsprovCharacter.ArbetsprovCharacter_C|SetObjectiveEnum _asarbetsprov_character "NewEnumerator1")
  (Actor|DestroyActor)
  (bind _asrocket_jump_game_mode (Utilities|Casting|CastToRocketJumpGameMode _returnvalue)
    (:then
      (Collision|SetActorEnableCollision (Variables|/Game/Arbetsprov/Blueprints/RocketJumpGameMode.RocketJumpGameMode_C|GetExtractionPointRef _asrocket_jump_game_mode) true)
      (Rendering|SetVisibility (Variables|/Game/Arbetsprov/Blueprints/ExtractionPoint.ExtractionPoint_C|GetSphere (Variables|/Game/Arbetsprov/Blueprints/RocketJumpGameMode.RocketJumpGameMode_C|GetExtractionPointRef _asrocket_jump_game_mode)) true false))
    (:CastFailed
      (bind _asarbetsprov_game_mode (Utilities|Casting|CastToArbetsprovGameMode _returnvalue))
      (Collision|SetActorEnableCollision (Variables|/Game/Arbetsprov/Blueprints/ArbetsprovGameMode.ArbetsprovGameMode_C|GetExtractionPointRef _asarbetsprov_game_mode) true)
      (Rendering|SetVisibility (Variables|/Game/Arbetsprov/Blueprints/ExtractionPoint.ExtractionPoint_C|GetSphere (Variables|/Game/Arbetsprov/Blueprints/ArbetsprovGameMode.ArbetsprovGameMode_C|GetExtractionPointRef _asarbetsprov_game_mode)) true false))))

(event EventTick
  (params (DeltaSeconds :type Float%20%28single-precision%29))
  (bind _cube (Variables|Default|GetCube))
  (bind _returnvalue (Transformation|GetWorldTransform _cube))
  (Utilities|FlowControl|Delay 0.01)
  (Transformation|SetWorldTransform _cube (Math|Transform|MakeTransform (.location _returnvalue) (Math|Rotator|MakeRotator (+ (.roll (.rotation _returnvalue)) 0.5) (.pitch (.rotation _returnvalue)) (.yaw (.rotation _returnvalue))) (.scale _returnvalue)) false false))

(fn ConstructionScript)